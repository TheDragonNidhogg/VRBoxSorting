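; Spawner actor for the timed level of the box sorting game that repeatedly spawns items at its own location.
; On BeginPlay it polls the game mode until StartGame, builds its item array from ItemNum, then loops spawns until PreFinished.
; The game instance sets the delay between spawns by speed index.
; Its FailRate sets the percentage chance of picking the first array entry instead of a random other one.
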(event EventBeginPlay
  (bind _assorting_game (Utilities|Casting|CastToSortingGame (Game|GetGameInstance)))
  (bind _astimed_game_mode (Utilities|Casting|CastToTimed_Game_Mode (Game|GetGameMode)))
  (if (Variables|/Game/BoxSortingGame/Time_Level_Standard/Timed_Game_Mode.Timed_Game_Mode_C|GetStart_Game _astimed_game_mode) :!label _label
    (CallFunction|CreateArraytoSpawn)
    (Utilities|ForLoop 0 (Variables|/Game/BoxSortingGame/SortingGame.SortingGame_C|GetItem_Num _assorting_game) 99 (Variables|/Game/BoxSortingGame/Time_Level_Standard/Timed_Game_Mode.Timed_Game_Mode_C|GetPre-Finished _astimed_game_mode) :!label _label_2
      (:LoopBody
        (CallFunction|Spawn))
      (:Delay%20Out
        (bind _assorting_game_2 (Utilities|Casting|CastToSortingGame (Game|GetGameInstance)))
        (Utilities|FlowControl|Delay (Utilities|Array|Get(acopy) (Variables|/Game/BoxSortingGame/SortingGame.SortingGame_C|GetDelay _assorting_game_2) (Variables|/Game/BoxSortingGame/SortingGame.SortingGame_C|GetSpeed%20Index _assorting_game_2)))
        (if (not (Variables|/Game/BoxSortingGame/Time_Level_Standard/Timed_Game_Mode.Timed_Game_Mode_C|GetPre-Finished _astimed_game_mode))
          (goto _label_2 Delay%20In))))
    (else
      (Utilities|FlowControl|Delay 0.1)
      (goto _label))))

(event Collision|EventActorBeginOverlap
  (params (OtherActor :type Actor%20Object%20Reference)))

(event EventTick
  (params (DeltaSeconds :type Float%20%28single-precision%29)))

(fn ConstructionScript)

(fn Spawn
  (bind _assorting_game (Utilities|Casting|CastToSortingGame (Game|GetGameInstance)))
  (Game|SpawnActorfromClass (Utilities|Array|Get(acopy) (Variables|Default|GetItemsToSpawn) (Math|Integer|SelectInt 0 (Math|Random|RandomIntegerinRange 1 (- (Utilities|Array|Length (Variables|Default|GetItemsToSpawn)) 1)) (< (Math|Random|RandomIntegerinRange 1 100) (Variables|/Game/BoxSortingGame/SortingGame.SortingGame_C|GetFail_Rate _assorting_game)))) (Math|Transform|MakeTransform (Transformation|GetActorLocation) (Transformation|GetActorRotation)) "AdjustIfPossibleButAlwaysSpawn" 0 0))

(fn CreateArraytoSpawn
  (switch int (Variables|Default|GetItem_Num)
    (:0
      (Variables|Default|SetItemsToSpawn (Variables|Default|GetItem1)))))