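; Game mode for the conveyor sorting game's level, tracking score and a round countdown.
; Events add or subtract points, and StartRound records a real-time start stamp.
; BeginPlay copies Started and Finished from the SortingGame game instance, and Tick polls Started until true.
; Tick then uses the Time function to derive minutes and seconds left from game time, setting the local Finished at zero.
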(event Custom|SubtractPoints
  (params (SubtractPoints :type Integer))
  (Variables|Default|SetScore (- (Variables|Default|GetScore) SubtractPoints)))

(event Custom|AddPoints
  (params (AddPoints :type Integer))
  (Variables|Default|SetScore (+ AddPoints (Variables|Default|GetScore))))

(event Custom|Start%20Round
  (Variables|Default|SetStart (Math|Float|Truncate (Utilities|Time|GetRealTimeSeconds))))

(event EventBeginPlay
  (Variables|Default|SetSeconds 0)
  (Variables|Default|SetMinutes 0)
  (bind _assorting_game (Utilities|Casting|CastToSortingGame (Game|GetGameInstance)))
  (Variables|Default|SetFinished (Variables|/Game/BoxSortingGame/SortingGame.SortingGame_C|GetFinished _assorting_game))
  (Variables|Default|SetStarted (Variables|/Game/BoxSortingGame/SortingGame.SortingGame_C|GetStarted _assorting_game)))

(event EventTick
  (params (DeltaSeconds :type Float%20%28single-precision%29))
  (if (Variables|Default|GetStarted)
    (bind (_minutes _seconds _done _time_in_seconds) (CallFunction|Time (Variables|Default|GetStart) (Variables|Default|GetTotal%20Time)))
    (if _done
      (Variables|Default|SetSeconds 0)
      (Variables|Default|SetMinutes 0)
      (Variables|Default|SetTimer _time_in_seconds)
      (Variables|Default|SetFinished true)
      (else
        (Variables|Default|SetSeconds _seconds)
        (Variables|Default|SetMinutes _minutes)))
    (else
      (bind _assorting_game (Utilities|Casting|CastToSortingGame (Game|GetGameInstance)))
      (Variables|Default|SetStarted (Variables|/Game/BoxSortingGame/SortingGame.SortingGame_C|GetStarted _assorting_game)))))

(fn ConstructionScript)

(fn Time
  (params (Start%20Time :type Integer) (Total%20Time :type Integer))
  (bind _returnvalue (Utilities|Time|GetGameTimeinSeconds))
  (bind _returnvalue_2 (Math|Float|Truncate _returnvalue))
  (bind _returnvalue_3 (- _returnvalue_2 Start%20Time))
  (bind _returnvalue_4 (- Total%20Time _returnvalue_3))
  (bind _returnvalue_5 (/ _returnvalue_4 60))
  (bind _returnvalue_6 (* _returnvalue_5 60))
  (bind _returnvalue_7 (- _returnvalue_4 _returnvalue_6))
  (if (and (<= _returnvalue_5 0) (<= _returnvalue_7 0))
    (return 0 0 true _returnvalue_4)
    (else
      (return _returnvalue_5 _returnvalue_7 false _returnvalue_4))))