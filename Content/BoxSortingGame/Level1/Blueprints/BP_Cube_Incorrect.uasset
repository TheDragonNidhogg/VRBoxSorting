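; BP_Cube_Incorrect is the incorrect-cube actor in Level 1 of the box sorting game, scoring itself when destroyed.
; On Destroyed, it checks for actors overlapping the first removal system, then the second if none are found.
; A first-system overlap subtracts Points times Multiplier from the SortingGame game instance's Score and increments Misses.
; A second-system overlap adds the same amount to Score.
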(event EventDestroyed
  (if (> (Utilities|Array|Length (Collision|GetOverlappingActors "/Game/BoxSortingGame/Level1/Blueprints/First_Removal_System.First_Removal_System_C" :!class /Script/Engine.Actor)) 0)
    (bind _assorting_game (Utilities|Casting|CastToSortingGame (Game|GetGameInstance)))
    (Variables|/Game/BoxSortingGame/SortingGame.SortingGame_C|SetScore _assorting_game (- (Variables|/Game/BoxSortingGame/SortingGame.SortingGame_C|GetScore _assorting_game) (* (Variables|Default|GetPoints) (Variables|Default|GetMultiplier))))
    (Variables|/Game/BoxSortingGame/SortingGame.SortingGame_C|SetMisses _assorting_game (+ (Variables|/Game/BoxSortingGame/SortingGame.SortingGame_C|GetMisses _assorting_game) 1))
    (elif (> (Utilities|Array|Length (Collision|GetOverlappingActors "/Game/BoxSortingGame/Level1/Blueprints/Second_Removal_System.Second_Removal_System_C" :!class /Script/Engine.Actor)) 0)
      (bind _assorting_game_2 (Utilities|Casting|CastToSortingGame (Game|GetGameInstance)))
      (Variables|/Game/BoxSortingGame/SortingGame.SortingGame_C|SetScore _assorting_game_2 (+ (Variables|/Game/BoxSortingGame/SortingGame.SortingGame_C|GetScore _assorting_game_2) (* (Variables|Default|GetPoints) (Variables|Default|GetMultiplier)))))))

(fn ConstructionScript
  (|CallParentFunction))