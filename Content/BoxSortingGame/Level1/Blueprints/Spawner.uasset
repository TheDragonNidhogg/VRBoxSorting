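; Spawner actor for the box sorting game's Level 1 that spawns random items at its own transform once the game starts.
; BeginPlay polls the SortingGame instance's Started flag, then fills ItemsToSpawn from Item1 when ItemNum is 0.
; A delay-driven loop, bounded by the ConveyorGameMode Timer, calls Spawn at two-second intervals.
; When the loop completes, it sets Finished on the game instance.
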(event EventBeginPlay
  (bind _assorting_game (Utilities|Casting|CastToSortingGame (Game|GetGameInstance)))
  (bind _asconveyor_game_mode (Utilities|Casting|CastToConveyorGameMode (Game|GetGameMode)))
  (Utilities|FlowControl|Delay 0.1 :!label _label)
  (if (Variables|/Game/BoxSortingGame/Level1/Blueprints/SortingGame.SortingGame_C|GetStarted _assorting_game)
    (CallFunction|CreateArraytoSpawn)
    (Utilities|ForLoop 0 (Variables|/Game/BoxSortingGame/Level1/Blueprints/SortingGame.SortingGame_C|GetItem_Num _assorting_game) (Variables|/Game/BoxSortingGame/Level1/Blueprints/ConveyorGameMode.ConveyorGameMode_C|GetTimer _asconveyor_game_mode) :!label _label_2
      (:LoopBody
        (CallFunction|Spawn))
      (:Completed
        (Variables|/Game/BoxSortingGame/Level1/Blueprints/SortingGame.SortingGame_C|SetFinished _assorting_game true))
      (:Delay%20Out
        (Utilities|FlowControl|Delay 2.0)
        (goto _label_2 Delay%20In)))
    (else
      (goto _label))))

(event Collision|EventActorBeginOverlap
  (params (OtherActor :type Actor%20Object%20Reference)))

(event EventTick
  (params (DeltaSeconds :type Float%20%28single-precision%29)))

(fn ConstructionScript)

(fn Spawn
  (Game|SpawnActorfromClass (Utilities|Array|Get(acopy) (Variables|Default|GetItemsToSpawn) (Math|Random|RandomIntegerinRange 0 (- (Utilities|Array|Length (Variables|Default|GetItemsToSpawn)) 1))) (Math|Transform|MakeTransform (Transformation|GetActorLocation) (Transformation|GetActorRotation)) "AdjustIfPossibleButAlwaysSpawn" 0 0))

(fn CreateArraytoSpawn
  (switch int (Variables|Default|GetItem_Num)
    (:0
      (Variables|Default|SetItemsToSpawn (Variables|Default|GetItem1)))))