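; Button1 is a physical start button for the box sorting Infinite Challenge level, pressed by a VR motion controller.
; When a BP_MotionController overlaps its Box, the Button component slides down via MoveComponentTo, and an end overlap slides it back up.
; After the press, it sets StartGame on Infinite_Challenge_Game_Mode, records the truncated real time as StartTimeInSeconds, then destroys itself.
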(event OnComponentBeginOverlap(Box)
  (params (OverlappedComponent :type Primitive%20Component%20Object%20Reference) (OtherActor :type Actor%20Object%20Reference) (OtherComp :type Primitive%20Component%20Object%20Reference) (OtherBodyIndex :type Integer) (bFromSweep :type Boolean) (SweepResult :type Hit%20Result%20Structure%20%28by%20ref%29))
  (bind _button (Variables|Default|GetButton))
  (bind _returnvalue (Transformation|GetRelativeTransform _button))
  (Utilities|Casting|CastToBP_MotionController OtherActor)
  (Components|MoveComponentTo _button (- (Math|Transform|TransformLocation _returnvalue "0, 0, 0") "0, 0,3.000000") (Math|Transform|TransformRotation _returnvalue "0, 0, 0") false false 1.0 false)
  (bind _asinfinite_challenge_game_mode (Utilities|Casting|CastToInfinite_Challenge_Game_Mode (Game|GetGameMode)))
  (Variables|/Game/BoxSortingGame/Infinite_Challenge_Level/Infinite_Challenge_Game_Mode.Infinite_Challenge_Game_Mode_C|SetStart_Game _asinfinite_challenge_game_mode true)
  (Variables|/Game/BoxSortingGame/Infinite_Challenge_Level/Infinite_Challenge_Game_Mode.Infinite_Challenge_Game_Mode_C|SetStart_Time_In_Seconds _asinfinite_challenge_game_mode (Math|Float|Truncate (Utilities|Time|GetRealTimeSeconds)))
  (Actor|DestroyActor))

(event OnComponentEndOverlap(Box)
  (params (OverlappedComponent :type Primitive%20Component%20Object%20Reference) (OtherActor :type Actor%20Object%20Reference) (OtherComp :type Primitive%20Component%20Object%20Reference) (OtherBodyIndex :type Integer))
  (bind _button (Variables|Default|GetButton))
  (bind _returnvalue (Transformation|GetRelativeTransform _button))
  (Utilities|Casting|CastToBP_MotionController OtherActor)
  (Components|MoveComponentTo _button (+ (Math|Transform|TransformLocation _returnvalue "0, 0, 0") "0, 0,3.000000") (Math|Transform|TransformRotation _returnvalue "0, 0, 0") false false 1.0 false))

(event EventBeginPlay)

(event Collision|EventActorBeginOverlap
  (params (OtherActor :type Actor%20Object%20Reference)))

(event EventTick
  (params (DeltaSeconds :type Float%20%28single-precision%29)))

(fn ConstructionScript)