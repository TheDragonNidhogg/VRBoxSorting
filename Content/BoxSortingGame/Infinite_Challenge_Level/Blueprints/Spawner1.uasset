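; Spawner actor for the Infinite Challenge level of the box sorting game, emitting items at its own transform.
; On BeginPlay it polls the SortingGame instance until started, then builds the item array from ItemNum.
; A delayed loop spawns items at intervals set by the current speed index, gated by the game mode's FinishedGame.
; Each spawn picks the array's first entry with FailRate percent odds, otherwise a random other entry.
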(event EventBeginPlay
  (bind _assorting_game (Utilities|Casting|CastToSortingGame (Game|GetGameInstance)))
  (bind _asinfinite_challenge_game_mode (Utilities|Casting|CastToInfinite_Challenge_Game_Mode (Game|GetGameMode)))
  (if (Variables|/Game/BoxSortingGame/SortingGame.SortingGame_C|GetStarted _assorting_game) :!label _label
    (CallFunction|CreateArraytoSpawn)
    (Utilities|ForLoop 0 (Variables|/Game/BoxSortingGame/SortingGame.SortingGame_C|GetItem_Num _assorting_game) 99 (Variables|/Game/BoxSortingGame/Infinite_Challenge_Level/Blueprints/Infinite_Challenge_Game_Mode.Infinite_Challenge_Game_Mode_C|GetFinished_Game _asinfinite_challenge_game_mode) :!label _label_2
      (:LoopBody
        (CallFunction|Spawn))
      (:Completed
        (Variables|/Game/BoxSortingGame/SortingGame.SortingGame_C|SetFinished _assorting_game true))
      (:Delay%20Out
        (bind _assorting_game_2 (Utilities|Casting|CastToSortingGame (Game|GetGameInstance)))
        (Utilities|FlowControl|Delay (Utilities|Array|Get(acopy) (Variables|/Game/BoxSortingGame/SortingGame.SortingGame_C|GetDelay _assorting_game_2) (Variables|/Game/BoxSortingGame/SortingGame.SortingGame_C|GetSpeed%20Index _assorting_game_2)))
        (if (not (Variables|/Game/BoxSortingGame/Infinite_Challenge_Level/Blueprints/Infinite_Challenge_Game_Mode.Infinite_Challenge_Game_Mode_C|GetFinished_Game _asinfinite_challenge_game_mode))
          (goto _label_2 Delay%20In))))
    (else
      (Utilities|FlowControl|Delay 0.1)
      (goto _label))))

(event Collision|EventActorBeginOverlap
  (params (OtherActor :type Actor%20Object%20Reference)))

(event EventTick
  (params (DeltaSeconds :type Float%20%28single-precision%29)))

(fn ConstructionScript)

(fn Spawn
  (bind _assorting_game (Utilities|Casting|CastToSortingGame (Game|GetGameInstance)))
  (Game|SpawnActorfromClass (Utilities|Array|Get(acopy) (Variables|Default|GetItemsToSpawn) (Math|Integer|SelectInt 0 (Math|Random|RandomIntegerinRange 1 (- (Utilities|Array|Length (Variables|Default|GetItemsToSpawn)) 1)) (< (Math|Random|RandomIntegerinRange 1 100) (Variables|/Game/BoxSortingGame/SortingGame.SortingGame_C|GetFail_Rate _assorting_game)))) (Math|Transform|MakeTransform (Transformation|GetActorLocation) (Transformation|GetActorRotation)) "AdjustIfPossibleButAlwaysSpawn" 0 0))

(fn CreateArraytoSpawn
  (switch int (Variables|Default|GetItem_Num)
    (:0
      (Variables|Default|SetItemsToSpawn (Variables|Default|GetItem1)))))